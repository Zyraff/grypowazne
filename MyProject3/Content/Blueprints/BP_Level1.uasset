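; BP_Level1 is a tile-map level that moves a robot across a grid through command functions returning success or failure.
; The construction script positions BPRobot using tile (0,0)'s transform and sets Heading to face right.
; TurnRight cycles four headings; MoveForward steps X/Y within map bounds and snaps the robot to the tile center without sweeping.
; CheckFront and PickUpItem are stubs returning false, and the event graph is empty.
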(fn `CheckFront`
  (returns (isClear :type Boolean))
  (return false))

(fn `MoveForward`
  (returns (IsMoved :type Boolean))
  (bind _tilemap (`PaperTileMapComponent.TileMap` (`self.Level1`)))
  (switch `int` (`self.Heading`)
    (:`0`
      (if (> (`self.x`) 0)
        (set `self.x` (+ (`self.x`) -1))
        (`SceneComponent.K2_SetRelativeLocation` (`self.BP_Robot`) (`PaperTileMapComponent.GetTileCenterPosition` (`self.Level1`) (`self.x`) (`self.y`) 0 true) false false :!label _label)
        (return true)
        (else
          _)))
    (:`1`
      (if (> (`self.y`) 0)
        (set `self.y` (+ (`self.y`) -1))
        (goto _label)
        (else
          _)))
    (:`2`
      (if (< (`self.x`) (- (`PaperTileMap.MapWidth` _tilemap) 1))
        (set `self.x` (+ (`self.x`) 1))
        (goto _label)
        (else
          _)))
    (:`3`
      (if (< (`self.y`) (- (`PaperTileMap.MapHeight` _tilemap) 1))
        (set `self.y` (+ (`self.y`) 1))
        (goto _label)
        (else
          _))))
  (return false))

(fn `PickUpItem`
  (returns (isPicked :type Boolean))
  (return false))

(fn `TurnRight`
  (returns (Success :type Boolean))
  (if (>= (`self.Heading`) 3)
    (set `self.Heading` 0)
    (else
      (set `self.Heading` (+ (`self.Heading`) 1))))
  (return true))

(fn `UserConstructionScript`
  (bind _returnvalue_location (`KismetMathLibrary.BreakTransform` (`TileMapBlueprintLibrary.GetTileTransform` (`PaperTileMapComponent.GetTile` (`self.Level1`) 0 0 0))))
  (`SceneComponent.K2_SetRelativeLocation` (`self.BP_Robot`) _returnvalue_location false false)
  (set `self.Heading` 2))